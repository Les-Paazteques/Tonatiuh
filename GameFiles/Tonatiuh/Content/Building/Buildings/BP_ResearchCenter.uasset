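; BP_ResearchCenter is a clickable research center building that opens its research HUD.
; On BeginPlay it binds its click event to ActivateUI, which creates a WBP_ResearchCenterHUD unless the stored one is already visible.
; Each new widget receives a reference to this building, is added to the viewport and takes focus in UI-only input mode.
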(event EventBeginPlay
  (EventDispatchers|BindEventtoOnClicked (delegate EventActivateUI)))

(event Collision|EventActorBeginOverlap
  (params (OtherActor :type Actor%20Object%20Reference)))

(event EventTick
  (params (DeltaSeconds :type Float%20%28single-precision%29)))

(event EventActivateUI
  (params (p_touchedActor :type Actor%20Object%20Reference) (p_keyPressed :type Key%20Structure :default "None"))
  (if (Utilities|IsValid (Variables|Default|GetWidget))
    (if (not (Widget|IsVisible (Variables|Default|GetWidget)))
      (bind _returnvalue (UserInterface|CreateWidget "/Game/UIs/BuildingUI/WBP_ResearchCenterHUD.WBP_ResearchCenterHUD_C" :!label _label))
      (Variables|/Game/UIs/BuildingUI/WBP_ResearchCenterHUD.WBP_ResearchCenterHUD_C|SetResearchCenter _returnvalue self)
      (UserInterface|Viewport|AddtoViewport _returnvalue 0)
      (bind _output_get (Variables|Default|SetWidget _returnvalue))
      (Input|SetInputModeUIOnly (Game|GetPlayerController 0) _output_get "DoNotLock" false))
    (else
      (goto _label))))

(fn ConstructionScript)