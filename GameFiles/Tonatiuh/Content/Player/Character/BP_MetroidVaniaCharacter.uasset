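; Player character Blueprint for the MetroidVania mode, managing its health and collectible HUD.
; On BeginPlay it adds both widgets to the viewport, hides the health bar and binds to BP_SwitchGamemode's MetroidVania and CityBuilder enter events.
; PlayerHealthComponent damage, max-health and death events refresh the health bar, and death also removes a collectible bar item.
; ActivateUI and DeactivateUI toggle only the health bar's visibility.
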(event OnDamaged(PlayerHealthComponent)
  (params (p_damageAmount :type Integer))
  (Default|SetHealth (Variables|Default|GetHealthBarUI)))

(event OnMaxHealthChange(PlayerHealthComponent)
  (params (p_healthAmount :type Integer))
  (Default|SetHealth (Variables|Default|GetHealthBarUI)))

(event OnDeath(PlayerHealthComponent)
  (Default|SetHealth (Variables|Default|GetHealthBarUI))
  (Default|RemoveItem (Variables|Default|GetCollectibleBarUI)))

(event EventBeginPlay
  (bind _returnvalue (UserInterface|CreateWidget "/Game/UIs/Collectible/WBP_CollectibleBar.WBP_CollectibleBar_C"))
  (bind _output_get (Variables|Default|SetCollectibleBarUI _returnvalue))
  (bind _returnvalue_2 (UserInterface|CreateWidget "/Game/Player/Health/UI/W_HealthBar.W_HealthBar_C" 0 self))
  (bind _output_get_2 (Variables|Default|SetHealthBarUI _returnvalue_2))
  (UserInterface|Viewport|AddtoViewport _output_get_2 0)
  (CallFunction|DeactivateUI)
  (bind _asbp_switch_gamemode (Utilities|Casting|CastToBP_SwitchGamemode (Game|GetGameMode)))
  (EventDispatchers|BindEventtoOnMetroidVaniaEnterEvent _asbp_switch_gamemode (EventDispatchers|CreateEvent :!event ActivateUI))
  (EventDispatchers|BindEventtoOnCityBuilderEnterEvent _asbp_switch_gamemode (EventDispatchers|CreateEvent :!event DeactivateUI)))

(event Collision|EventActorBeginOverlap
  (params (OtherActor :type Actor%20Object%20Reference)))

(event EventTick
  (params (DeltaSeconds :type Float%20%28single-precision%29)))

(fn ConstructionScript)

(fn DeactivateUI
  (Widget|SetVisibility (Variables|Default|GetHealthBarUI) "Hidden"))

(fn ActivateUI
  (Widget|SetVisibility (Variables|Default|GetHealthBarUI) "Visible"))