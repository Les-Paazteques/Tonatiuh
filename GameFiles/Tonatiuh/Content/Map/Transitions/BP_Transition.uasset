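; BP_Transition is a map trigger actor that changes game state when a BP_MetroidVaniaCharacter overlaps it.
; It forwards the action to BP_SwitchGamemode, chosen by its variables.
; A golem unlock with a named room takes priority and ends the flow.
; Otherwise it either switches to the city builder or loads or unloads the specified level.
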(event EventBeginPlay)

(event Collision|EventActorBeginOverlap
  (params (OtherActor :type Actor%20Object%20Reference))
  (bind _returnvalue (Game|GetGameMode))
  (bind _leveltoload (Variables|Default|GetLevelToLoad))
  (bind _golemroom (Variables|Default|GetGolemRoom))
  (Utilities|Casting|CastToBP_MetroidVaniaCharacter OtherActor)
  (if (Utilities|IsValid _returnvalue)
    (bind _asbp_switch_gamemode (Utilities|Casting|CastToBP_SwitchGamemode _returnvalue))
    (if (Variables|Default|GetUnlockGolem)
      (if (!= _golemroom "")
        (Class|SwitchGamemode|UnlockGolem _asbp_switch_gamemode _golemroom)
        (else
          (if (Variables|Default|GetToCity) :!label _label
            (Class|SwitchGamemode|SwitchtoCityBuilder _asbp_switch_gamemode)
            (elif (Variables|Default|GetLoad)
              (Class|SwitchGamemode|LoadLevel _asbp_switch_gamemode _leveltoload)
              (else
                (Class|SwitchGamemode|UnLoadLevel _asbp_switch_gamemode _leveltoload))))))
      (else
        (goto _label)))))

(event EventTick
  (params (DeltaSeconds :type Float%20%28single-precision%29)))

(fn ConstructionScript)