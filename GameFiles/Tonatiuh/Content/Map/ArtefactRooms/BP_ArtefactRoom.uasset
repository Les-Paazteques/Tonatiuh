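; BP_ArtefactRoom is a trigger actor that manages a character's temporary hold on the room's ContainedArtefact power-up until it is unlocked.
; On overlap begin, it calls AddPowerUp if the artefact is not unlocked and HasPowerUp returns true.
; On overlap end, it removes a still-locked power-up and always shows the Warning text.
; The warning widget is created on BeginPlay, and a Tick countdown clears its text.
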(event EventBeginPlay
  (bind _returnvalue (UserInterface|CreateWidget "/Game/UIs/WBP_ArtefactWarning.WBP_ArtefactWarning_C"))
  (bind _output_get (Variables|Default|SetArtefactWarning _returnvalue))
  (UserInterface|Viewport|AddtoViewport _output_get 0)
  (Class|NightWarningWidget|ResetText _output_get))

(event Collision|EventActorBeginOverlap
  (params (OtherActor :type Actor%20Object%20Reference))
  (bind _containedartefact (Variables|Default|GetContainedArtefact))
  (bind _asbp_metroid_vania_character (Utilities|Casting|CastToBP_MetroidVaniaCharacter OtherActor))
  (bind _returnvalue (Class|MetroidVaniaCharacter|HasUnlockedPowerUp _asbp_metroid_vania_character _containedartefact))
  (if (not _returnvalue)
    (bind _returnvalue_2 (Class|MetroidVaniaCharacter|HasPowerUp _asbp_metroid_vania_character _containedartefact))
    (if _returnvalue_2
      (Class|MetroidVaniaCharacter|AddPowerUp _asbp_metroid_vania_character _containedartefact))))

(event EventTick
  (params (DeltaSeconds :type Float%20%28single-precision%29))
  (if (> (Variables|Default|Gettimer) 0.0)
    (bind _output_get (Variables|Default|Settimer (- (Variables|Default|Gettimer) DeltaSeconds)))
    (if (<= _output_get 0.0)
      (Class|NightWarningWidget|ResetText (Variables|Default|GetArtefactWarning)))))

(event Collision|EventActorEndOverlap
  (params (OtherActor :type Actor%20Object%20Reference))
  (bind _asbp_metroid_vania_character (Utilities|Casting|CastToBP_MetroidVaniaCharacter OtherActor))
  (Class|NightWarningWidget|SetText (Variables|Default|GetArtefactWarning) (Variables|Default|GetWarning))
  (Variables|Default|Settimer 1e+01)
  (bind _returnvalue (Class|MetroidVaniaCharacter|HasUnlockedPowerUp _asbp_metroid_vania_character (Variables|Default|GetContainedArtefact)))
  (if (not _returnvalue)
    (Class|MetroidVaniaCharacter|RemovePowerUp _asbp_metroid_vania_character (Variables|Default|GetContainedArtefact))))

(fn ConstructionScript)